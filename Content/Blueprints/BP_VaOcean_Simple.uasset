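; BP_VaOcean_Simple is an ocean actor that renders water through a simple dynamic material on its static mesh.
; On BeginPlay it creates the material instance and fills its wave height, panning, UV scaling and water height parameters from the actor's getters.
; Each Tick it feeds game time into the wave height panner, so the material animates on the same clock as gameplay.
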(event EventBeginPlay
  (bind _self self)
  ;[1 1 1] Ocean material
  (bind _returnvalue (Rendering|Material|CreateDynamicMaterialInstance "/VaOcean/MatInsts/M_OceanSimple_Inst.M_OceanSimple_Inst" :!class /Script/Engine.KismetMaterialLibrary))
  (Variables|Default|SetOceanMaterial _returnvalue)
  (Rendering|Material|SetMaterial (Variables|Default|GetStaticMesh1) 0 (Variables|Default|GetOceanMaterial))
  ;[1 1 1] Ocean instance setup
  (Rendering|Material|SetScalarParameterValue (Variables|Default|GetOceanMaterial) "WorldPositionDivider" (Class|VaOceanStateActorSimple|GetWorldPositionDivider _self) :!class /Script/Engine.MaterialInstanceDynamic)
  (Rendering|Material|SetScalarParameterValue (Variables|Default|GetOceanMaterial) "WaveUVDivider" (Class|VaOceanStateActorSimple|GetWaveUVDivider _self) :!class /Script/Engine.MaterialInstanceDynamic)
  (Rendering|Material|SetScalarParameterValue (Variables|Default|GetOceanMaterial) "WaveHeightPannerX" (Class|VaOceanStateActorSimple|GetWaveHeightPannerX _self) :!class /Script/Engine.MaterialInstanceDynamic)
  (Rendering|Material|SetScalarParameterValue (Variables|Default|GetOceanMaterial) "WaveHeightPannerY" (Class|VaOceanStateActorSimple|GetWaveHeightPannerY _self) :!class /Script/Engine.MaterialInstanceDynamic)
  (Rendering|Material|SetScalarParameterValue (Variables|Default|GetOceanMaterial) "WaveHeight" (Class|VaOceanStateActorSimple|GetWaveHeight _self) :!class /Script/Engine.MaterialInstanceDynamic)
  (Rendering|Material|SetScalarParameterValue (Variables|Default|GetOceanMaterial) "WaterHeight" (Class|VaOceanStateActorSimple|GetWaterHeight _self) :!class /Script/Engine.MaterialInstanceDynamic))

(event EventTick
  (params (DeltaSeconds :type Float%20%28single-precision%29))
  (Rendering|Material|SetScalarParameterValue (Variables|Default|GetOceanMaterial) "WaveHeightPannerTime" (Utilities|Time|GetGameTimeinSeconds) :!class /Script/Engine.MaterialInstanceDynamic))

(fn ConstructionScript)